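; BP_Projectile is a cannon projectile that damages the actors it touches.
; On BeginPlay it launches its Sphere component with a physics impulse taken from the Impulse variable.
; Sphere hit and begin-overlap events each apply their own fixed damage to the other actor, with no type filter.
; A character cast and a DestroyActor call are left unconnected, so the projectile never destroys itself in this graph.
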(event OnComponentHit(Sphere)
  (params (HitComponent :type Primitive%20Component%20Object%20Reference) (OtherActor :type Actor%20Object%20Reference) (OtherComp :type Primitive%20Component%20Object%20Reference) (NormalImpulse :type Vector :default "0, 0, 0") (Hit :type Hit%20Result%20Structure%20%28by%20ref%29))
  (Game|Damage|ApplyDamage OtherActor 1e+01 0 self))

(event OnComponentBeginOverlap(Sphere)
  (params (OverlappedComponent :type Primitive%20Component%20Object%20Reference) (OtherActor :type Actor%20Object%20Reference) (OtherComp :type Primitive%20Component%20Object%20Reference) (OtherBodyIndex :type Integer) (bFromSweep :type Boolean) (SweepResult :type Hit%20Result%20Structure%20%28by%20ref%29))
  (Game|Damage|ApplyDamage OtherActor 18.0 0 self))

(event EventBeginPlay
  (Physics|AddImpulse (Variables|Default|GetSphere) (Variables|Default|GetImpulse) "None" false))

(fn ConstructionScript)