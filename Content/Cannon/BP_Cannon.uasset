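; BP_Cannon is a turret that tracks the third-person character and fires projectiles while it sees them.
; PawnSensing stores the character and sets a visibility flag, cleared after roughly one sensing interval.
; Tick smoothly turns the actor in yaw only and fires through a DoOnce reset after a short delay.
; Each shot plays an explosion sound and spawns BP_Projectile with an impulse along the muzzle's up vector.
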(event OnSeePawn(PawnSensing)
  (params (Pawn :type Pawn%20Object%20Reference))
  (bind _asbp_third_person_character (Utilities|Casting|CastToBP_ThirdPersonCharacter Pawn))
  (Variables|Default|SetAs%20BP%20Third%20Person%20Character _asbp_third_person_character)
  (Variables|Default|SetCanSeePlayer true)
  (Utilities|FlowControl|Delay (- (Variables|/Script/AIModule.PawnSensingComponent|GetSensingInterval (Variables|Default|GetPawnSensing)) (Class|Actor|GetActorTickInterval)))
  (Variables|Default|SetCanSeePlayer false))

(event EventBeginPlay)

(event Collision|EventActorBeginOverlap
  (params (OtherActor :type Actor%20Object%20Reference)))

(event EventTick
  (params (DeltaSeconds :type Float%20%28single-precision%29))
  (bind _returnvalue (Transformation|GetActorRotation))
  (bind _as_bp_third_person_character (Variables|Default|GetAs%20BP%20Third%20Person%20Character))
  (Utilities|IsValid _as_bp_third_person_character
    (:Is%20Valid
      (if (Variables|Default|GetCanSeePlayer)
        (Transformation|SetActorRotation (Math|Interpolation|RInterpTo (Transformation|GetActorRotation) (Math|Rotator|MakeRotator (.roll _returnvalue) (.pitch _returnvalue) (.yaw (Math|Rotator|FindLookatRotation (Transformation|GetActorLocation) (Transformation|GetActorLocation _as_bp_third_person_character)))) (Utilities|Time|GetWorldDeltaSeconds) 5.0))
        (Utilities|FlowControl|DoOnce false :!label _label
          (:Completed
            (Utilities|FlowControl|Sequence
              (:then_0
                (Audio|PlaySoundatLocation "/Game/StarterContent/Audio/Explosion_Cue.Explosion_Cue" (Transformation|GetActorLocation) "0, 0, 0" 1.0 1.0 0.0 0 0 0 0)
                (Game|SpawnActorfromClass "/Game/Cannon/BP_Projectile.BP_Projectile_C" (Math|Transform|MakeTransform (Transformation|GetWorldLocation (Variables|Default|GetSpawnPoint)) "0, 0, 0" "1.000000,1.000000,1.000000") "Undefined" 0 (* (Math|Vector|GetUpVector (Variables|Default|GetMuzzle)) (Variables|Default|GetFireStrength)) 0))
              (:then_1
                (Utilities|FlowControl|Delay 1.0)
                (goto _label Reset)))))))))

(fn ConstructionScript
  (Transformation|SetWorldRotation (Variables|Default|GetBase) "0, 0, 0" false false))